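; BP_HISMTestActor is a test actor that slides along the world X axis at a constant speed.
; Each Tick offsets its location by a fixed velocity scaled by delta time, without sweeping.
; An unconnected chain would ask the BattlefieldManagerSubsystem's manager actor to spawn a static mesh tagged as an allied army unit owned by this actor, but it never runs.
; BeginPlay only waits one tick.
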(event `self.ReceiveBeginPlay`
  (`KismetSystemLibrary.DelayUntilNextTick`))

(event `self.ReceiveTick`
  (params (DeltaSeconds :type "Float (single-precision)"))
  (`self.K2_SetActorLocation` (+ (`self.K2_GetActorLocation`) (* (`GameplayStatics.GetWorldDeltaSeconds`) (100.0 0.0 0.0)))))

(fn `UserConstructionScript`)