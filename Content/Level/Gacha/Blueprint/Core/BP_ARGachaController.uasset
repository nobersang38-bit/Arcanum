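; BP_ARGachaController drives the scripted camera move for the AR gacha sequence.
; StartCameraSequence chains three timelines, each lerping GachaCamera between hardcoded world positions: a rise from below, a settle to mid height, then a push in along X.
; When the last timeline finishes, it calls EndCameraSequence.
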(event `self.StartCameraSequence`
  (bind (_direction _newtrack_0) (`Timeline|TL_CameraDownUp` :!via `PlayFromStart`)
    (:`Update`
      (`self.K2_SetActorLocation` (`self.GachaCamera`) (`KismetMathLibrary.VLerp` (-2800.0 -9980.0 -400.0) (-2800.0 -9940.0 400.0) _newtrack_0) false false))
    (:`Finished`
      (bind (_direction_2 _newtrack_0_2) (`Timeline|TL_CameraUpMidle` :!via `PlayFromStart`)
        (:`Update`
          (`self.K2_SetActorLocation` (`self.GachaCamera`) (`KismetMathLibrary.VLerp` (-2800.0 -9980.0 400.0) (-2800.0 -9940.0 200.0) _newtrack_0_2) false false))
        (:`Finished`
          (bind (_direction_3 _newtrack_0_3) (`Timeline|TL_CameraMiddleZoomUp` :!via `PlayFromStart`)
            (:`Update`
              (`self.K2_SetActorLocation` (`self.GachaCamera`) (`KismetMathLibrary.VLerp` (-2800.0 -9980.0 200.0) (-2120.0 -9940.0 10.0) _newtrack_0_3) false false))
            (:`Finished`
              (`self.EndCameraSequence`))))))))

(fn `UserConstructionScript`)